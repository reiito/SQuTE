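; Game mode for a local two-player Rock-Paper-Scissors game where losing a round costs health until one player reaches zero.
; BeginPlay creates the second local player and HUD, caches PlayerStarts for pawn respawning, and initializes health and timer.
; While GameRunning, Tick counts down each round, resolving it when both players choose or time expires.
; Results update health and text, then a DoOnce-guarded delay resets the round.
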(event `self.ReceiveBeginPlay`
  (`self.SetReferences`)
  (`self.InitVariables`))

(event `self.ReceiveTick`
  (params (DeltaSeconds :type "Float (single-precision)"))
  (if (`self.GameRunning`)
    (bind (_gameover _p1wins) (`self.CheckGameOver`))
    (if _gameover
      (if _p1wins
        (set `self.StateText` "Player 1 Wins The Game!")
        (else
          (set `self.StateText` "Player 2 Wins The Game!")))
      (set `self.GameRunning` false)
      (elif (`self.RoundEnd`)
        (`/Engine/EditorBlueprintResources/StandardMacros.DoOnce` false :!label _label
          (:`Completed`
            (`KismetSystemLibrary.Delay` (`self.DelayDuration`))
            (`self.ResetRound`)))
        (else
          (`self.RoundTimer`)
          (`self.RestartRound`))))))

(event `RestartRound`
  (goto _label :!via `Reset`))

(event `SpawnPlayer`
  (params (PlayerController :type "PlayerController Object Reference"))
  (bind _returnvalue (`Controller.K2_GetPawn` PlayerController))
  (bind _returnvalue_2 (`GameplayStatics.GetPlayerControllerID` PlayerController))
  (`/Engine/EditorBlueprintResources/StandardMacros.IsValid` _returnvalue
    (:`Is Valid`
      (`self.K2_DestroyActor` _returnvalue)
      (bind _returnvalue_3 (`|SpawnActorFromClass` "/Game/Blueprints/BP_Player.BP_Player_C" (`self.GetTransform` (`|GetArrayItem` (`self.SpawnPoints`) _returnvalue_2)) "Undefined" "OverrideRootScale" null null))
      (`Controller.Possess` PlayerController _returnvalue_3))))

(event `Key|Escape`
  (params (Key :type "Key Structure"))
  (:`Pressed`
    (`KismetSystemLibrary.QuitGame` null "Quit")))

(fn `CheckBothDone`
  (returns (Ready :type Boolean))
  (return (and (`|EnumInequality` (`self.P1Choice`) "NewEnumerator3") (`|EnumInequality` (`self.P2Choice`) "NewEnumerator3"))))

(fn `CheckGameOver`
  (returns (GameOver :type Boolean) (P1Wins :type Boolean))
  (bind _returnvalue (<= (`self.P2Health`) 0.0))
  (return (or (<= (`self.P1Health`) 0.0) _returnvalue) _returnvalue))

(fn `EvaluateRound`
  (bind _p2choice (`self.P2Choice`))
  (if (`|EnumEquality` (`self.P1Choice`) (`self.P2Choice`))
    (set `self.Result` "NewEnumerator0")
    (elif (`|EnumEquality` (`self.P2Choice`) "NewEnumerator3")
      (set `self.Result` "NewEnumerator1")
      (else
        (switch `/Game/Data/ENUM_Choices` (`self.P1Choice`)
          (:`NewEnumerator3`
            (set `self.Result` "NewEnumerator2" :!label _label))
          (:`NewEnumerator0`
            (if (`|EnumEquality` _p2choice "NewEnumerator2")
              (set `self.Result` "NewEnumerator1" :!label _label_2)
              (else
                (goto _label))))
          (:`NewEnumerator1`
            (if (`|EnumEquality` _p2choice "NewEnumerator0")
              (goto _label_2)
              (else
                (goto _label))))
          (:`NewEnumerator2`
            (if (`|EnumEquality` _p2choice "NewEnumerator1")
              (goto _label_2)
              (else
                (goto _label)))))))))

(fn `InitVariables`
  (bind _maxhealth (`self.MaxHealth`))
  (set `self.P1Health` _maxhealth)
  (set `self.P2Health` _maxhealth)
  (set `self.CurrentRoundTime` (`self.RoundDuration`))
  (set `self.StateText` "Press Enter To Start"))

(fn `P1Text`
  (switch `/Game/Data/ENUM_Choices` (`self.P1Choice`)
    (:`NewEnumerator3`
      (set `self.P1RockText` "")
      (set `self.P1PaperText` "")
      (set `self.P1ScissorsText` ""))
    (:`NewEnumerator0`
      (set `self.P1PaperText` "")
      (set `self.P1ScissorsText` ""))
    (:`NewEnumerator1`
      (set `self.P1RockText` "")
      (set `self.P1ScissorsText` ""))
    (:`NewEnumerator2`
      (set `self.P1RockText` "")
      (set `self.P1PaperText` ""))))

(fn `P2Text`
  (switch `/Game/Data/ENUM_Choices` (`self.P2Choice`)
    (:`NewEnumerator3`
      (set `self.P2RockText` "")
      (set `self.P2PaperText` "")
      (set `self.P2ScissorsText` ""))
    (:`NewEnumerator0`
      (set `self.P2PaperText` "")
      (set `self.P2ScissorsText` ""))
    (:`NewEnumerator1`
      (set `self.P2RockText` "")
      (set `self.P2ScissorsText` ""))
    (:`NewEnumerator2`
      (set `self.P2RockText` "")
      (set `self.P2PaperText` ""))))

(fn `ResetRound`
  (bind _roundduration (`self.RoundDuration`))
  (set `self.P1InputDis` false)
  (set `self.P2InputDis` false)
  (set `self.CurrentRoundTime` _roundduration)
  (set `self.CurrentHUDTime` (/ _roundduration _roundduration))
  (`self.ResetText`)
  (set `self.P1Choice` "NewEnumerator3")
  (set `self.P2Choice` "NewEnumerator3")
  (set `self.Result` "NewEnumerator0")
  (set `self.RoundEnd` false))

(fn `ResetStates`)

(fn `ResetText`
  (set `self.P1RockText` "Rock")
  (set `self.P1PaperText` "Paper")
  (set `self.P1ScissorsText` "Scissors")
  (set `self.P2RockText` "Rock")
  (set `self.P2PaperText` "Paper")
  (set `self.P2ScissorsText` "Scissors"))

(fn `RoundTimer`
  (bind _returnvalue (- (`self.CurrentRoundTime`) (`GameplayStatics.GetWorldDeltaSeconds`)))
  (if (> (`self.CurrentRoundTime`) 0.0)
    (set `self.CurrentRoundTime` _returnvalue)
    (set `self.CurrentHUDTime` (`KismetMathLibrary.FClamp` (/ _returnvalue (`self.RoundDuration`))))
    (bind _ready (`self.CheckBothDone`))
    (if _ready
      (`self.EvaluateRound` :!label _label)
      (`self.RoundWinBehaviour`))
    (else
      (goto _label))))

(fn `RoundWinBehaviour`
  (switch `/Game/Data/ENUM_Result` (`self.Result`)
    (:`NewEnumerator0`
      (set `self.StateText` "This Round Was A Draw"))
    (:`NewEnumerator1`
      (set `self.StateText` "Player 1 Wins The Round")
      (set `self.P2Health` (- (`self.P2Health`) (`self.Damage`))))
    (:`NewEnumerator2`
      (set `self.StateText` "Player 2 Wins The Round")
      (set `self.P1Health` (- (`self.P1Health`) (`self.Damage`)))))
  (`self.P1Text`)
  (`self.P2Text`)
  (set `self.RoundEnd` true))

(fn `SetReferences`
  (`|ExecutionSequence`
    (:`then_0`
      (bind _outactors (`GameplayStatics.GetAllActorsOfClass` "/Script/Engine.PlayerStart"))
      (set `self.SpawnPoints` _outactors))
    (:`then_1`
      (set `self.P1Reference` (`GameplayStatics.GetPlayerController` 0))
      (bind _returnvalue (`GameplayStatics.CreatePlayer` -1))
      (set `self.P2Reference` _returnvalue))
    (:`then_2`
      (bind _returnvalue_2 (`|CreateWidget` "/Game/Blueprints/BP_GameHUD.BP_GameHUD_C"))
      (bind _output_get (set `self.HUDReference` _returnvalue_2))
      (`UserWidget.AddToViewport` _output_get 0))))

(fn `UserConstructionScript`)