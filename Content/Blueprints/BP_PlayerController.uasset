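; Player controller for a local two-player rock-paper-scissors game, writing each player's choice to BP_GameMode.
; Controller ID splits Player 1 keyboard and Player 2 gamepad picks, accepted only while the game runs and that player's choice is empty.
; A pick sets that player's input-disabled flag, which Tick polls to toggle input; Enter or gamepad Special Right starts the game through DoOnce.
; Uncalled P1Text and P2Text helpers blank choice labels.
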(event `self.ReceiveBeginPlay`
  (bind _asbp_game_mode (cast `/Game/Blueprints/BP_GameMode` (`GameplayStatics.GetGameMode`)))
  (set `self.GameModeReference` _asbp_game_mode))

(event `self.ReceiveTick`
  (params (DeltaSeconds :type "Float (single-precision)"))
  (bind _gamemodereference (`self.GameModeReference`))
  (bind _returnvalue (`GameplayStatics.GetPlayerControllerID` self))
  (switch `int` _returnvalue
    (:`0`
      (if (`/Game/Blueprints/BP_GameMode.P1InputDis` _gamemodereference)
        (`self.DisableInput` self :!label _label)
        (else
          (`self.EnableInput` self :!label _label_2))))
    (:`1`
      (if (`/Game/Blueprints/BP_GameMode.P2InputDis` _gamemodereference)
        (goto _label)
        (else
          (goto _label_2))))))

(event `Key|Z`
  (params (Key :type "Key Structure"))
  (bind _gamemodereference (`self.GameModeReference`))
  (:`Pressed`
    (bind _valid (`self.P1Valid`))
    (if _valid
      (set `/Game/Blueprints/BP_GameMode.P1Choice` "NewEnumerator0" _gamemodereference)
      (set `/Game/Blueprints/BP_GameMode.P1InputDis` true _gamemodereference :!label _label_3))))

(event `Key|X`
  (params (Key :type "Key Structure"))
  (:`Pressed`
    (bind _valid (`self.P1Valid`))
    (if _valid
      (set `/Game/Blueprints/BP_GameMode.P1Choice` "NewEnumerator1" (`self.GameModeReference`))
      (goto _label_3))))

(event `Key|C`
  (params (Key :type "Key Structure"))
  (:`Pressed`
    (bind _valid (`self.P1Valid`))
    (if _valid
      (set `/Game/Blueprints/BP_GameMode.P1Choice` "NewEnumerator2" (`self.GameModeReference`))
      (goto _label_3))))

(event `Key|Gamepad_FaceButton_Left`
  (params (Key :type "Key Structure"))
  (bind _gamemodereference (`self.GameModeReference`))
  (:`Pressed`
    (bind _valid (`self.P2Valid`))
    (if _valid
      (set `/Game/Blueprints/BP_GameMode.P2Choice` "NewEnumerator0" _gamemodereference)
      (set `/Game/Blueprints/BP_GameMode.P2InputDis` true _gamemodereference :!label _label_4))))

(event `Key|Gamepad_FaceButton_Bottom`
  (params (Key :type "Key Structure"))
  (:`Pressed`
    (bind _valid (`self.P2Valid`))
    (if _valid
      (set `/Game/Blueprints/BP_GameMode.P2Choice` "NewEnumerator1" (`self.GameModeReference`))
      (goto _label_4))))

(event `Key|Gamepad_FaceButton_Right`
  (params (Key :type "Key Structure"))
  (:`Pressed`
    (bind _valid (`self.P2Valid`))
    (if _valid
      (set `/Game/Blueprints/BP_GameMode.P2Choice` "NewEnumerator2" (`self.GameModeReference`))
      (goto _label_4))))

(event `Key|Enter`
  (params (Key :type "Key Structure"))
  (:`Pressed`
    (`/Engine/EditorBlueprintResources/StandardMacros.DoOnce` false :!label _label_5
      (:`Completed`
        (set `/Game/Blueprints/BP_GameMode.GameRunning` true (`self.GameModeReference`))))))

(event `Key|Gamepad_Special_Right`
  (params (Key :type "Key Structure"))
  (:`Pressed`
    (goto _label_5)))

(fn `P1Text`
  (params (Choice :type "/Game/Data/ENUM_Choices Enum" :default "NewEnumerator3"))
  (bind _gamemodereference (`self.GameModeReference`))
  (switch `/Game/Data/ENUM_Choices` Choice
    (:`NewEnumerator0`
      (set `/Game/Blueprints/BP_GameMode.P2PaperText` "" _gamemodereference)
      (set `/Game/Blueprints/BP_GameMode.P1ScissorsText` "" _gamemodereference))
    (:`NewEnumerator1`
      (set `/Game/Blueprints/BP_GameMode.P1RockText` "" _gamemodereference)
      (set `/Game/Blueprints/BP_GameMode.P1ScissorsText` "" _gamemodereference))
    (:`NewEnumerator2`
      (set `/Game/Blueprints/BP_GameMode.P1RockText` "" _gamemodereference)
      (set `/Game/Blueprints/BP_GameMode.P2PaperText` "" _gamemodereference))))

(fn `P1Valid`
  (returns (Valid :type Boolean))
  (bind _gamemodereference (`self.GameModeReference`))
  (bind _returnvalue (`GameplayStatics.GetPlayerControllerID` self))
  (switch `int` _returnvalue
    (:`0`
      (if (`|EnumEquality` (`/Game/Blueprints/BP_GameMode.P1Choice` _gamemodereference) "NewEnumerator3")
        (if (`/Game/Blueprints/BP_GameMode.GameRunning` _gamemodereference)
          (return true)
          (else
            _))))
    (:`1`
      _))
  (return false))

(fn `P2Text`
  (params (Choice :type "/Game/Data/ENUM_Choices Enum" :default "NewEnumerator3"))
  (bind _gamemodereference (`self.GameModeReference`))
  (switch `/Game/Data/ENUM_Choices` Choice
    (:`NewEnumerator0`
      (set `/Game/Blueprints/BP_GameMode.P2PaperText` "" _gamemodereference)
      (set `/Game/Blueprints/BP_GameMode.P2ScissorsText` "" _gamemodereference))
    (:`NewEnumerator1`
      (set `/Game/Blueprints/BP_GameMode.P2RockText` "" _gamemodereference)
      (set `/Game/Blueprints/BP_GameMode.P2ScissorsText` "" _gamemodereference))
    (:`NewEnumerator2`
      (set `/Game/Blueprints/BP_GameMode.P2RockText` "" _gamemodereference)
      (set `/Game/Blueprints/BP_GameMode.P2PaperText` "" _gamemodereference))))

(fn `P2Valid`
  (returns (Valid :type Boolean))
  (bind _gamemodereference (`self.GameModeReference`))
  (bind _returnvalue (`GameplayStatics.GetPlayerControllerID` self))
  (switch `int` _returnvalue
    (:`0`
      _)
    (:`1`
      (if (`|EnumEquality` (`/Game/Blueprints/BP_GameMode.P2Choice` _gamemodereference) "NewEnumerator3")
        (if (`/Game/Blueprints/BP_GameMode.GameRunning` _gamemodereference)
          (return true)
          (else
            _)))))
  (return false))

(fn `UserConstructionScript`)